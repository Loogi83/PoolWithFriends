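; Spline tool Blueprint in the pool table folder that lays a chosen static mesh along an editable spline.
; The construction script divides the spline length by SectionLength and adds a spline mesh component per section, applying the mesh, forward axis and collision type.
; GetStartEndPosition samples local positions and tangents by distance, clamping tangent size to the section length.
; The event graph is unused.
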(fn `GetStartEndPosition`
  (params (Index :type Integer))
  (returns (Position :type "Vector Structure") (Tangent :type "Vector Structure"))
  (bind _spline (`self.Spline`))
  (bind _returnvalue (* Index (`self.SectionLength`)))
  (return (`SplineComponent.GetLocationAtDistanceAlongSpline` _spline _returnvalue "Local") (`KismetMathLibrary.ClampVectorSize` (`SplineComponent.GetTangentAtDistanceAlongSpline` _spline _returnvalue "Local") 0.0 (`self.SectionLength`))))

(fn `UserConstructionScript`
  (locals (LoopIndex :type Integer))
  (bind (_position _tangent) (`self.GetStartEndPosition` (`local.LoopIndex`)))
  (bind (_position_2 _tangent_2) (`self.GetStartEndPosition` (+ (`local.LoopIndex`) 1)))
  (for _index (range (+ (`KismetMathLibrary.FTrunc` (/ (`SplineComponent.GetSplineLength` (`self.Spline`)) (`self.SectionLength`))) 1))
    (set `local.LoopIndex` _index)
    (bind _returnvalue (`AddComponent|NODE_AddSplineMeshComponent-0`))
    (`StaticMeshComponent.SetStaticMesh` _returnvalue (`self.Mesh`))
    (`SplineMeshComponent.SetForwardAxis` _returnvalue (`self.In Forward Axis`) true)
    (`SplineMeshComponent.SetStartAndEnd` _returnvalue _position _tangent _position_2 _tangent_2 true)
    (`PrimitiveComponent.SetCollisionEnabled` _returnvalue (`self.CollisionType`))))