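; BP_Pocket_Collider is a pool table pocket trigger that detects physics-body balls entering its box and plays a pocket sound.
; A potted BP_DummyBall prints its number and notifies GM_Pool through BallPotted, while a potted BP_PlayerBall respawns.
; It binds to the game mode's table-complete dispatcher to set an Ignore flag, which skips the next player ball respawn and then clears.
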(event `self.ReceiveBeginPlay`
  (bind _asgm_pool (cast `/Game/PoolWithFriends/Core/GameModes/GM_Pool` (`GameplayStatics.GetGameMode`)))
  (bind _output_get (set `self.As GM Pool` _asgm_pool))
  (add `/Game/PoolWithFriends/Core/GameModes/GM_Pool.ED_TableComplete` _output_get (`|CreateDelegate` :!event `OnTableComplete`)))

(event `self.Box.OnComponentBeginOverlap`
  (params (OverlappedComponent :type "PrimitiveComponent Object Reference") (OtherActor :type "Actor Object Reference") (OtherComp :type "PrimitiveComponent Object Reference") (OtherBodyIndex :type Integer) (bFromSweep :type Boolean) (SweepResult :type "HitResult Structure (by ref)"))
  (switch `ECollisionChannel` (`PrimitiveComponent.GetCollisionObjectType` OtherComp)
    (:`ECC_PhysicsBody`
      (`GameplayStatics.PlaySoundAtLocation` "/Game/PoolWithFriends/Balls/Common/Audio/SW_Pocket.SW_Pocket" (`self.K2_GetActorLocation`) (struct) 1.0 1.0 0.0 null null null null)
      (bind _asbp_dummy_ball (cast `/Game/PoolWithFriends/Balls/Dummy/BP_DummyBall` OtherActor)
        (:`then`
          (`KismetSystemLibrary.PrintString` (`KismetTextLibrary.Conv_TextToString` (`|FormatText` "Ball Number {Number} Potted!" (`/Game/PoolWithFriends/Balls/Dummy/BP_DummyBall.Number` _asbp_dummy_ball))))
          (`/Game/PoolWithFriends/Core/GameModes/GM_Pool.BallPotted` (`self.As GM Pool`)))
        (:`CastFailed`
          (bind _asbp_player_ball (cast `/Game/PoolWithFriends/Core/PlayerBall/BP_PlayerBall` OtherActor))
          (if (not (`self.Ignore`))
            (`/Game/PoolWithFriends/Core/PlayerBall/BP_PlayerBall.RespawnBall` _asbp_player_ball)
            (else
              (set `self.Ignore` false))))))))

(event `OnTableComplete`
  (set `self.Ignore` true))

(fn `UserConstructionScript`)