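; BP_DummyBall is a numbered pool ball that colours itself and plays impact sounds.
; The construction script picks one of eight colours from Number, applying M_Base to the first material slot for numbers above 8 to separate stripes from solids.
; Blocking sphere hits record LastValidLocation, then play ball or wall sounds by collision object type with speed-scaled volume.
; Floor hits play a 2D wall sound only with enough upward velocity.
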(event `self.Sphere.OnComponentHit`
  (params (HitComponent :type "PrimitiveComponent Object Reference") (OtherActor :type "Actor Object Reference") (OtherComp :type "PrimitiveComponent Object Reference") (NormalImpulse :type "Vector Structure") (Hit :type "HitResult Structure (by ref)"))
  (bind (_bblockinghit _binitialoverlap _time _distance _location _impactpoint _normal _impactnormal _physmat _hitactor _hitcomponent) (`GameplayStatics.BreakHitResult` Hit))
  (bind _returnvalue (`self.K2_GetActorLocation`))
  (bind (_returnvalue_x _returnvalue_y _returnvalue_z) (`KismetMathLibrary.BreakVector` (`self.GetVelocity`)))
  (bind _returnvalue_2 (`KismetMathLibrary.NormalizeToRange` (`KismetMathLibrary.VSize` (`self.GetVelocity`)) 0.0 300.0))
  (if _bblockinghit
    (set `self.LastValidLocation` (`self.K2_GetActorLocation`))
    (if (>= _returnvalue_2 0.1)
      (switch `ECollisionChannel` (`PrimitiveComponent.GetCollisionObjectType` _hitcomponent)
        (:`ECC_PhysicsBody`
          (`GameplayStatics.PlaySoundAtLocation` "/Game/PoolWithFriends/Balls/Common/Audio/SC_BallHit.SC_BallHit" _returnvalue (struct) _returnvalue_2 1.0 0.0 null null null null))
        (:`ECC_GameTraceChannel1`
          (`GameplayStatics.PlaySoundAtLocation` "/Game/PoolWithFriends/Balls/Common/Audio/SC_Wall.SC_Wall" _returnvalue (struct) _returnvalue_2 1.0 0.0 null null null null))
        (:`ECC_GameTraceChannel2`
          (if (> _returnvalue_z 50.0)
            (`GameplayStatics.PlaySound2D` "/Game/PoolWithFriends/Balls/Common/Audio/SC_Wall.SC_Wall" 1.0 1.0 0.0 null null false)))))))

(fn `UserConstructionScript`
  (bind _sphere (`self.Sphere`))
  (`PrimitiveComponent.SetMaterial` _sphere 1 (select `int` (- (`self.Number`) (`KismetMathLibrary.SelectInt` 9 1 (> (`self.Number`) 8))) :`0` "/Game/PoolWithFriends/Balls/Dummy/MI_Base_Yellow.MI_Base_Yellow" :`1` "/Game/PoolWithFriends/Balls/Dummy/MI_Base_Blue.MI_Base_Blue" :`2` "/Game/PoolWithFriends/Balls/Dummy/M_Accent.M_Accent" :`3` "/Game/PoolWithFriends/Balls/Dummy/MI_Base_Purple.MI_Base_Purple" :`4` "/Game/PoolWithFriends/Balls/Dummy/MI_Base_Orange.MI_Base_Orange" :`5` "/Game/PoolWithFriends/Balls/Dummy/MI_Base_Green.MI_Base_Green" :`6` "/Game/PoolWithFriends/Balls/Dummy/MI_Base_Brown.MI_Base_Brown" :`7` "/Game/PoolWithFriends/Balls/Dummy/MI_Base_Black.MI_Base_Black" :!type "MaterialInterface Object Reference"))
  (`PrimitiveComponent.SetMaterial` (`self.Sphere`) 0 (select `bool` (> (`self.Number`) 8) :`false` (`PrimitiveComponent.GetMaterial` _sphere 1) :`true` "/Game/PoolWithFriends/Balls/Dummy/M_Base.M_Base")))