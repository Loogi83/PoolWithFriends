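; GM_Pool is the pool game mode that tracks how many balls remain on the table.
; On BeginPlay it counts every BP_DummyBall actor and stores that as both the default and remaining count.
; BallPotted decrements the count and, at zero or below, calls the TableComplete event dispatcher and prints a message.
; ResetBalls restores the count to the stored default.
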(event `self.ReceiveBeginPlay`
  (bind _outactors (`GameplayStatics.GetAllActorsOfClass` "/Game/PoolWithFriends/Balls/Dummy/BP_DummyBall.BP_DummyBall_C"))
  (bind _output_get (set `self.DefaultNumber` (`KismetArrayLibrary.Array_Length` _outactors)))
  (set `self.BallsRemaining` _output_get))

(event `BallPotted`
  (bind _result (`/Engine/EditorBlueprintResources/StandardMacros.DecrementInt` (`self.BallsRemaining`))
    (:`  `
      (if (<= _result 0)
        (`self.ED_TableComplete`)
        (`KismetSystemLibrary.PrintString` "Table Complete")))))

(event `ResetBalls`
  (set `self.BallsRemaining` (`self.DefaultNumber`)))

(fn `UserConstructionScript`)