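; BP_Pocket_Collider is a pool table pocket trigger that detects balls dropping in.
; Its sphere's radius is set from a variable in the construction script.
; When a Physics Body component overlaps the sphere, it plays the pocket sound at the actor's location.
; If the actor is a BP_DummyBall, it prints a debug message with the potted ball's number, with no scoring or ball removal here.
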(event `self.Sphere.OnComponentBeginOverlap`
  (params (OverlappedComponent :type "PrimitiveComponent Object Reference") (OtherActor :type "Actor Object Reference") (OtherComp :type "PrimitiveComponent Object Reference") (OtherBodyIndex :type Integer) (bFromSweep :type Boolean) (SweepResult :type "HitResult Structure (by ref)"))
  (switch `ECollisionChannel` (`PrimitiveComponent.GetCollisionObjectType` OtherComp)
    (:`ECC_PhysicsBody`
      (`GameplayStatics.PlaySoundAtLocation` "/Game/PoolWithFriends/Balls/Common/Audio/SW_Pocket.SW_Pocket" (`self.K2_GetActorLocation`) (struct) 1.0 1.0 0.0 null null null null)
      (bind _asbp_dummy_ball (cast `/Game/PoolWithFriends/Balls/Dummy/BP_DummyBall` OtherActor))
      (`KismetSystemLibrary.PrintString` (`KismetTextLibrary.Conv_TextToString` (`|FormatText` "Ball Number {Number} Potted!" (`/Game/PoolWithFriends/Balls/Dummy/BP_DummyBall.Number` _asbp_dummy_ball)))))))

(fn `UserConstructionScript`
  (`SphereComponent.SetSphereRadius` (`self.Sphere`) (`self.In Sphere Radius`) true))