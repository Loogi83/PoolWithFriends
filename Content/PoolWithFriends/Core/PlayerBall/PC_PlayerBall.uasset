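; Player controller for the pool player ball, handling camera look, cue aiming, power and shots.
; A looping mouse trace positions the cue on the controlled ball, and click-and-drag builds clamped power shown on the cue and HUD.
; Release applies a camera-forward impulse at the clicked point, flattening Z unless aimed steeply downward.
; A velocity-polling timer tracks ball movement, blocking shots and restarting aiming once it stops.
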(event `self.ReceiveBeginPlay`
  (bind _returnvalue (subsystem `EnhancedInputLocalPlayerSubsystem`))
  ;[1 1 1] Begin Play
  (`EnhancedInputSubsystemInterface.AddMappingContext` _returnvalue "/Game/PoolWithFriends/Core/Input/IMC_BallControls.IMC_BallControls" 0 (struct))
  (`EnhancedInputSubsystemInterface.AddMappingContext` _returnvalue "/Game/PoolWithFriends/Core/Input/IMC_Cue.IMC_Cue" 1 (struct))
  (bind _returnvalue_2 (`|CreateWidget` "/Game/PoolWithFriends/Core/Widgets/W_Power.W_Power_C"))
  (bind _output_get (set `self.PowerHUD` _returnvalue_2))
  (`UserWidget.AddToViewport` _output_get 0)
  (`self.CueTrace`))

(event `self.ReceivePossess`
  (params (PossessedPawn :type "Pawn Object Reference"))
  ;[1 1 1] Get and Set camera Variable
  (bind _asbp_player_ball (cast `/Game/PoolWithFriends/Core/PlayerBall/BP_PlayerBall` PossessedPawn))
  (bind _output_get (set `self.PlayerBall` _asbp_player_ball))
  (set `self.PlayerCamera` (`/Game/PoolWithFriends/Core/PlayerBall/BP_PlayerBall.Camera` _output_get)))

(event `EnhancedInput|/Game/PoolWithFriends/Core/Input/IA_Look`
  (params (ActionValue :type "Vector2D Structure") (ElapsedSeconds :type "Float (double-precision)") (TriggeredSeconds :type "Float (double-precision)") (InputAction :type "InputAction Object Reference" :default "/Game/PoolWithFriends/Core/Input/IA_Look.IA_Look"))
  (bind _returnvalue (`self.K2_GetPawn`))
  (bind _tracetimerhandle (`self.TraceTimerHandle`))
  ;[1 1 1] Look
  (:`Triggered`
    (if (`self.CanLook?`)
      (`Pawn.AddControllerYawInput` _returnvalue ActionValue_X)
      (`Pawn.AddControllerPitchInput` _returnvalue (* ActionValue_Y (`KismetMathLibrary.SelectFloat` 1.0 -1.0 (`self.invertCamera?`))))))
  (:`Started`
    (set `self.bShowMouseCursor` false)
    (`KismetSystemLibrary.K2_PauseTimerHandle` _tracetimerhandle))
  (:`Completed`
    (set `self.bShowMouseCursor` true)
    (`KismetSystemLibrary.K2_UnPauseTimerHandle` _tracetimerhandle)))

(event `CueTrace`
  ;[1 1 1] Trace and Calculate Cue placement
  (bind _returnvalue (`KismetSystemLibrary.K2_SetTimerDelegate` (delegate `UpdateTrace`) 0.01 true))
  (set `self.TraceTimerHandle` _returnvalue))

(event `UpdateTrace`
  (bind (_worldlocation _worlddirection) (`self.DeprojectMousePositionToWorld`))
  ;[1 1 1] Trace and Calculate Cue placement
  (bind (_outhit _returnvalue) (`KismetSystemLibrary.LineTraceSingleForObjects` :`Start` _worldlocation :`End` (+ _worldlocation (* _worlddirection (`self.TraceLength`))) :`ObjectTypes` (`|MakeArray` "ObjectTypeQuery4" "ObjectTypeQuery8" "ObjectTypeQuery7" :!type "EObjectTypeQuery Enum") :`DrawTime` 0.0))
  (if _returnvalue
    (bind (_bblockinghit _binitialoverlap _time _distance _location _impactpoint _normal _impactnormal _physmat _hitactor _hitcomponent) (`GameplayStatics.BreakHitResult` _outhit))
    (if (== _hitactor (`self.K2_GetPawn`))
      (set `self.Hit Component` _hitcomponent)
      (`/Game/PoolWithFriends/Core/PlayerBall/BP_PlayerBall.UpdateCueLocation` (`self.PlayerBall`) _location))))

(event `EnhancedInput|/Game/PoolWithFriends/Core/Input/IA_Click`
  (params (ActionValue :type Boolean) (ElapsedSeconds :type "Float (double-precision)") (TriggeredSeconds :type "Float (double-precision)") (InputAction :type "InputAction Object Reference" :default "/Game/PoolWithFriends/Core/Input/IA_Click.IA_Click"))
  ;[1 1 1] Trace and Calculate Cue placement
  (:`Started`
    (`/Engine/EditorBlueprintResources/StandardMacros.IsValid` (`self.Hit Component`)
      (:`Is Valid`
        (`KismetSystemLibrary.K2_PauseTimerHandle` (`self.TraceTimerHandle`))
        (set `self.CanLook?` false)
        (set `self.ImpactPoint` (`.Location` (`GameplayStatics.BreakHitResult` (stale `UpdateTrace` _outhit))))))))

(event `EnhancedInput|/Game/PoolWithFriends/Core/Input/IA_Click`
  (params (ActionValue :type Boolean) (ElapsedSeconds :type "Float (double-precision)") (TriggeredSeconds :type "Float (double-precision)") (InputAction :type "InputAction Object Reference" :default "/Game/PoolWithFriends/Core/Input/IA_Click.IA_Click"))
  (bind _hit_component (`self.Hit Component`))
  (bind _returnvalue (`KismetMathLibrary.NormalizeToRange` (`self.CurrentPower`) 0.0 (`self.MaxPower`)))
  (bind (_returnvalue_x _returnvalue_y _returnvalue_z) (`KismetMathLibrary.BreakVector` (`SceneComponent.GetForwardVector` (`self.PlayerCamera`))))
  ;[1 1 1] Shoot Ball at Cue Location
  (:`Completed`
    (if (not (`self.IsBallMoving?`))
      (`/Engine/EditorBlueprintResources/StandardMacros.IsValid` _hit_component
        (:`Is Valid`
          (`KismetSystemLibrary.K2_ClearAndInvalidateTimerHandle` (`self.TraceTimerHandle`))
          (`self.OnBallShot`)
          (set `self.CanLook?` true)
          (if (>= _returnvalue 0.1)
            (`GameplayStatics.PlaySound2D` "/Game/PoolWithFriends/Balls/Common/Audio/SC_CueHit.SC_CueHit" _returnvalue 1.0 0.0 null null false))
          (`PrimitiveComponent.AddImpulseAtLocation` _hit_component (* (`KismetMathLibrary.MakeVector` _returnvalue_x _returnvalue_y (`KismetMathLibrary.SelectFloat` 0.0 _returnvalue_z (> _returnvalue_z -0.3))) (`self.CurrentPower`)) (`self.ImpactPoint`) "None")
          (set `self.ImpactPoint` (0.0 0.0 0.0))
          (set `self.CurrentPower` 0.0)
          (set `self.Hit Component` null)
          (bind _returnvalue_2 (`KismetSystemLibrary.K2_SetTimerDelegate` (`|CreateDelegate` :!event `StopCheck`) 0.1 true))
          (set `self.StopCheckHandle` _returnvalue_2))))))

(event `StopCheck`
  ;[1 1 1] Stop Check
  (if (`KismetMathLibrary.Vector_IsNearlyZero` (`self.GetVelocity` (`self.K2_GetPawn`)) (`self.StopTolerance`))
    (set `self.IsBallMoving?` false)
    (`self.OnBallStop`)
    (`self.CueTrace`)
    (`KismetSystemLibrary.K2_ClearAndInvalidateTimerHandle` (`self.StopCheckHandle`))
    (else
      (set `self.IsBallMoving?` true)
      (`KismetSystemLibrary.K2_PauseTimerHandle` (`self.TraceTimerHandle`)))))

(event `EnhancedInput|/Game/PoolWithFriends/Core/Input/IA_Drag`
  (params (ActionValue :type "Float (double-precision)") (ElapsedSeconds :type "Float (double-precision)") (TriggeredSeconds :type "Float (double-precision)") (InputAction :type "InputAction Object Reference" :default "/Game/PoolWithFriends/Core/Input/IA_Drag.IA_Drag"))
  ;[1 1 1] Drag Cue
  (:`Triggered`
    (`/Engine/EditorBlueprintResources/StandardMacros.IsValid` (`self.Hit Component`)
      (:`Is Valid`
        (if (not (`self.IsBallMoving?`))
          (bind _output_get (set `self.CurrentPower` (`KismetMathLibrary.FClamp` (+ (`self.CurrentPower`) (* ActionValue (`self.PullMultiplier`))) 0.0 (`self.MaxPower`))))
          (`/Game/PoolWithFriends/Core/Widgets/W_Power.SetPercent` (`self.PowerHUD`) _output_get (`self.MaxPower`))
          (`/Game/PoolWithFriends/Core/PlayerBall/BP_PlayerBall.UpdateCueDistance` (`self.PlayerBall`) (`self.CurrentPower`) (`self.MaxPower`)))))))

(fn `UserConstructionScript`)