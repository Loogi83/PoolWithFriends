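; BP_DummyBall is a pool ball actor with no event logic that takes its look from its Number.
; The construction script maps Number to one of eight color materials on the Sphere's second slot, so 9 and up reuse the colors from 1 onward.
; The first slot gets M_Base for numbers above 8 and otherwise copies the color, producing striped or solid balls.
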(fn `UserConstructionScript`
  (bind _sphere (`self.Sphere`))
  (`PrimitiveComponent.SetMaterial` _sphere 1 (select `int` (- (`self.Number`) (`KismetMathLibrary.SelectInt` 9 1 (> (`self.Number`) 8))) :`0` "/Game/PoolWithFriends/Core/PlayerBall/MI_Base_Yellow.MI_Base_Yellow" :`1` "/Game/PoolWithFriends/Core/PlayerBall/MI_Base_Blue.MI_Base_Blue" :`2` "/Game/PoolWithFriends/Core/PlayerBall/M_Accent.M_Accent" :`3` "/Game/PoolWithFriends/Core/PlayerBall/MI_Base_Purple.MI_Base_Purple" :`4` "/Game/PoolWithFriends/Core/PlayerBall/MI_Base_Orange.MI_Base_Orange" :`5` "/Game/PoolWithFriends/Core/PlayerBall/MI_Base_Green.MI_Base_Green" :`6` "/Game/PoolWithFriends/Core/PlayerBall/MI_Base_Brown.MI_Base_Brown" :`7` "/Game/PoolWithFriends/Core/PlayerBall/MI_Base_Black.MI_Base_Black" :!type "MaterialInterface Object Reference"))
  (`PrimitiveComponent.SetMaterial` (`self.Sphere`) 0 (select `bool` (> (`self.Number`) 8) :`false` (`PrimitiveComponent.GetMaterial` _sphere 1) :`true` "/Game/PoolWithFriends/Core/PlayerBall/M_Base.M_Base")))