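; Player cue ball for a pool game, handling aim preview, cue and circle indicator, camera effects and impact sounds.
; PC_PlayerBall shot and stop events toggle aiming visuals, and each stop saves the location the R key respawns to.
; Looping timers replace Tick, driving a sphere-traced ghost ball, speed-based FOV during shots and smoothed zoom.
; Hit sounds depend on surface and speed; an air-check trace exists but is not connected.
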(event `self.ReceivePossessed`
  (params (NewController :type "Controller Object Reference"))
  (bind _aspc_player_ball (cast `/Game/PoolWithFriends/Core/PlayerBall/PC_PlayerBall` NewController))
  (add `/Game/PoolWithFriends/Core/PlayerBall/PC_PlayerBall.OnBallShot` _aspc_player_ball (`|CreateDelegate` :!event `OnBallShot`))
  (add `/Game/PoolWithFriends/Core/PlayerBall/PC_PlayerBall.OnBallStop` _aspc_player_ball (`|CreateDelegate` :!event `OnBallStop`))
  (`self.AimTrace`)
  (set `self.LastValidLocation` (`self.K2_GetActorLocation`)))

(event `Key|R`
  (params (Key :type "Key Structure"))
  (:`Pressed`
    (`self.RespawnBall`)))

(event `AirCheck`
  ;[1 1 1] Is Ball in Air
  (bind _returnvalue (`KismetSystemLibrary.K2_SetTimerDelegate` (delegate `UpdateAirTrace`) 0.1 true))
  (set `self.AirHandle` _returnvalue))

(event `EnhancedInput|/Game/PoolWithFriends/Core/Input/IA_Zoom`
  (params (ActionValue :type "Float (double-precision)") (ElapsedSeconds :type "Float (double-precision)") (TriggeredSeconds :type "Float (double-precision)") (InputAction :type "InputAction Object Reference" :default "/Game/PoolWithFriends/Core/Input/IA_Zoom.IA_Zoom"))
  ;[1 1 1] Camera Zoom
  (:`Triggered`
    (set `self.TargetCameraDistance` (`KismetMathLibrary.FClamp` (+ (`SpringArmComponent.TargetArmLength` (`self.CameraBoom`)) (* ActionValue (`self.ZoomSpeed`))) (`self.MinCameraDistance`) (`self.MaxCameraDistance`)))
    (if (not (`KismetSystemLibrary.K2_IsTimerActiveHandle` (`self.ZoomHandle`)))
      (bind _returnvalue (`KismetSystemLibrary.K2_SetTimerDelegate` (`|CreateDelegate` :!event `UpdateCameraDistance`) 0.01 true))
      (set `self.ZoomHandle` _returnvalue))))

(event `UpdateAirTrace`
  (bind _returnvalue (`self.K2_GetActorLocation`))
  ;[1 1 1] Is Ball in Air
  (bind (_outhit _returnvalue_2) (`KismetSystemLibrary.LineTraceSingleForObjects` :`Start` _returnvalue :`End` (- _returnvalue (0.0 0.0 100.0)) :`ObjectTypes` (`|MakeArray` "ObjectTypeQuery8" :!type "EObjectTypeQuery Enum") :`DrawDebugType` "ForDuration" :`DrawTime` 1.0))
  (if (!= _returnvalue_2 (`self.OnFloor?`))
    (set `self.OnFloor?` _returnvalue_2)))

(event `HideCue`
  ;[1 1 1] Pool Cue
  (`SceneComponent.SetVisibility` (`self.CueMesh`) false false))

(event `ShowCircle`
  ;[1 1 1] Circle Indicator
  (`SceneComponent.SetVisibility` (`self.Plane`) true false)
  (bind (_direction _scale) (`Timeline|EnterCircle` :!via `PlayFromStart`)
    (:`Update`
      (`SceneComponent.SetRelativeScale3D` (`self.Plane`) (* (`self.PlaneRelativeScale`) _scale)))))

(event `UpdateCueLocation`
  (params (NewLocation :type "Vector Structure"))
  ;[1 1 1] Pool Cue
  (`SceneComponent.K2_SetWorldLocationAndRotation` (`self.CuePlacer`) NewLocation (`SceneComponent.K2_GetComponentRotation` (`self.Camera`)) false false))

(event `FOV`
  ;[1 1 1] FOV
  (bind _returnvalue (`KismetSystemLibrary.K2_SetTimerDelegate` (delegate `UpdateFOV`) 0.01 true))
  (set `self.FOVHandle` _returnvalue))

(event `HideCircle`
  ;[1 1 1] Circle Indicator
  (`SceneComponent.SetVisibility` (`self.Plane`) false false))

(event `ShowCue`
  ;[1 1 1] Pool Cue
  (`SceneComponent.SetVisibility` (`self.CueMesh`) true false))

(event `UpdateFOV`
  ;[1 1 1] FOV
  (`CameraComponent.SetFieldOfView` (`self.Camera`) (`KismetMathLibrary.FInterpTo` (`CameraComponent.FieldOfView` (`self.Camera`)) (`KismetMathLibrary.MapRangeClamped` (`KismetMathLibrary.VSize` (`self.GetVelocity`)) 0.0 3000.0 90.0 120.0) (`GameplayStatics.GetWorldDeltaSeconds`) 5.0)))

(event `OnBallStop`
  ;[1 1 1] OnBallStop
  (`self.ShowCircle`)
  (`self.ShowCue`)
  (`self.AimTrace`)
  (set `self.LastValidLocation` (`self.K2_GetActorLocation`))
  (`KismetSystemLibrary.K2_ClearAndInvalidateTimerHandle` (`self.FOVHandle`)))

(event `UpdateCueDistance`
  (params (Power :type "Float (double-precision)") (MaxPower :type "Float (double-precision)"))
  ;[1 1 1] Pool Cue
  (set `SpringArmComponent.TargetArmLength` (`KismetMathLibrary.MapRangeClamped` Power 0.0 MaxPower 0.0 (`self.MaxCueDistance`)) (`self.CuePlacer`)))

(event `OnBallShot`
  ;[1 1 1] OnBallShot
  (`self.HideCircle`)
  (`self.HideCue`)
  (set `SpringArmComponent.TargetArmLength` 0.0 (`self.CuePlacer`))
  (`KismetSystemLibrary.K2_ClearAndInvalidateTimerHandle` (`self.AimHandle`))
  (`SceneComponent.SetVisibility` (`self.GhostBall`) false false)
  (`self.FOV`))

(event `self.Sphere.OnComponentHit`
  (params (HitComponent :type "PrimitiveComponent Object Reference") (OtherActor :type "Actor Object Reference") (OtherComp :type "PrimitiveComponent Object Reference") (NormalImpulse :type "Vector Structure") (Hit :type "HitResult Structure (by ref)"))
  (bind (_bblockinghit _binitialoverlap _time _distance _location _impactpoint _normal _impactnormal _physmat _hitactor _hitcomponent) (`GameplayStatics.BreakHitResult` Hit))
  (bind (_returnvalue_x _returnvalue_y _returnvalue_z) (`KismetMathLibrary.BreakVector` (`self.GetVelocity`)))
  (bind _returnvalue (`KismetMathLibrary.NormalizeToRange` (`KismetMathLibrary.VSize` (`self.GetVelocity`)) 0.0 300.0))
  ;[1 1 1] Hit Sounds
  (if _bblockinghit
    (if (>= _returnvalue 0.1)
      (switch `ECollisionChannel` (`PrimitiveComponent.GetCollisionObjectType` _hitcomponent)
        (:`ECC_PhysicsBody`
          (`GameplayStatics.PlaySound2D` "/Game/PoolWithFriends/Balls/Common/Audio/SC_BallHit.SC_BallHit" _returnvalue 1.0 0.0 null null false))
        (:`ECC_GameTraceChannel1`
          (`GameplayStatics.PlaySound2D` "/Game/PoolWithFriends/Balls/Common/Audio/SC_Wall.SC_Wall" _returnvalue 1.0 0.0 null null false))
        (:`ECC_GameTraceChannel2`
          (if (> _returnvalue_z 50.0)
            (`GameplayStatics.PlaySound2D` "/Game/PoolWithFriends/Balls/Common/Audio/SC_Wall.SC_Wall" 1.0 1.0 0.0 null null false)))))))

(event `AimTrace`
  ;[1 1 1] Aiming
  (bind _returnvalue (`KismetSystemLibrary.K2_SetTimerDelegate` (delegate `UpdateAim`) 0.01 true))
  (set `self.AimHandle` _returnvalue))

(event `UpdateAim`
  (bind _returnvalue (`self.K2_GetActorLocation`))
  (bind (_returnvalue_x _returnvalue_y _returnvalue_z) (`KismetMathLibrary.BreakVector` (`SceneComponent.GetForwardVector` (`self.Camera`))))
  ;[1 1 1] Aiming
  (bind (_outhit _returnvalue_2) (`KismetSystemLibrary.SphereTraceSingleForObjects` _returnvalue (+ _returnvalue (* (`KismetMathLibrary.MakeVector` _returnvalue_x _returnvalue_y (`KismetMathLibrary.SelectFloat` 0.0 _returnvalue_z (> _returnvalue_z -0.3))) 5000.0)) 45.0 (`|MakeArray` "ObjectTypeQuery4" "ObjectTypeQuery7" "ObjectTypeQuery8" :!type "EObjectTypeQuery Enum") false (`|MakeArray` self :!type "Actor Object Reference")))
  (`|ExecutionSequence`
    (:`then_0`
      (if (!= (`SceneComponent.bVisible` (`self.GhostBall`)) _returnvalue_2)
        (`SceneComponent.SetVisibility` (`self.GhostBall`) _returnvalue_2 false)))
    (:`then_1`
      (if _returnvalue_2
        (`SceneComponent.K2_SetWorldLocation` (`self.GhostBall`) (`.Location` (`GameplayStatics.BreakHitResult` _outhit)) false false)))))

(fn `RespawnBall`
  (bind _sphere (`self.Sphere`))
  (`PrimitiveComponent.SetPhysicsLinearVelocity` _sphere (0.0 0.0 0.0) false "None")
  (`PrimitiveComponent.SetPhysicsAngularVelocityInDegrees` _sphere (0.0 0.0 0.0) false "None")
  (`self.K2_SetActorLocation` (`self.LastValidLocation`)))

(fn `UpdateCameraDistance`
  (locals (ErrorTolerance :type "Float (double-precision)" :default 0.1) (CameraInterpSpeed :type "Float (double-precision)" :default 2.0))
  (bind _output_get (set `SpringArmComponent.TargetArmLength` (`KismetMathLibrary.FInterpTo` (`SpringArmComponent.TargetArmLength` (`self.CameraBoom`)) (`self.TargetCameraDistance`) (`GameplayStatics.GetWorldDeltaSeconds`) (`local.CameraInterpSpeed`)) (`self.CameraBoom`)))
  (if (`KismetMathLibrary.NearlyEqual_FloatFloat` _output_get (`self.TargetCameraDistance`) (`local.ErrorTolerance`))
    (`KismetSystemLibrary.K2_ClearAndInvalidateTimerHandle` (`self.ZoomHandle`))))

(fn `UserConstructionScript`
  (set `self.PlaneRelativeScale` (`SceneComponent.RelativeScale3D` (`self.Plane`))))